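; Pressure button for the level program pack that stays pressed while at least one actor overlaps its Box.
; Overlap begin and end update the Actors list, then ProvNaj toggles the Zaj pressed flag only when occupancy changes.
; Each change swaps the Paper2D sprite and sends ButtonsSig or ButtonsNoSig with the button's Name to the OSWidget on the player pawn's HUD.
; BeginPlay assigns its sprite component to the PaperSprite variable.
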(event OnComponentBeginOverlap(Box)
  (params (OverlappedComponent :type Primitive%20Component%20Object%20Reference) (OtherActor :type Actor%20Object%20Reference) (OtherComp :type Primitive%20Component%20Object%20Reference) (OtherBodyIndex :type Integer) (bFromSweep :type Boolean) (SweepResult :type Hit%20Result%20Structure%20%28by%20ref%29))
  (Utilities|Array|Add (Variables|Default|GetActors) OtherActor)
  (CallFunction|ProvNaj))

(event OnComponentEndOverlap(Box)
  (params (OverlappedComponent :type Primitive%20Component%20Object%20Reference) (OtherActor :type Actor%20Object%20Reference) (OtherComp :type Primitive%20Component%20Object%20Reference) (OtherBodyIndex :type Integer))
  (Utilities|Array|RemoveItem (Variables|Default|GetActors) OtherActor)
  (CallFunction|ProvNaj))

(event Custom|ProvNaj
  (bind _returnvalue (Game|Player|GetPlayerPawn 0))
  (bind _name (Variables|Default|GetName))
  (bind _returnvalue_2 (Utilities|String|ToString(Text) _name))
  (bind _astt_cum (Utilities|Casting|CastToTT_Cum _returnvalue))
  (bind _hud (Variables|/Game/Blueprints/Character/Player/TT_Cum.TT_Cum_C|GetHUD _astt_cum))
  (bind _os_widget (Variables|/Game/Blueprints/Character/Player/OS_hud.OS_hud_C|GetOS_Widget _hud))
  (if (== (Utilities|Array|Length (Variables|Default|GetActors)) 0)
    (if (Variables|Default|GetZaj?)
      (Variables|Default|SetZaj? false)
      (Rendering|Components|Sprite|SetSprite (Variables|Default|GetPaperSprite1) "/Game/2D-Sprites/Button2_Sprite.Button2_Sprite")
      (Default|ButtonsNoSig _os_widget _returnvalue_2))
    (elif (not (Variables|Default|GetZaj?))
      (Variables|Default|SetZaj? true)
      (Rendering|Components|Sprite|SetSprite (Variables|Default|GetPaperSprite1) "/Game/2D-Sprites/Buttton1_Sprite.Buttton1_Sprite")
      (Default|ButtonsSig _os_widget _returnvalue_2))))

(event EventBeginPlay
  ;[1 1 1] Обязательная для всех
  (Variables|Default|SetPaperSprite (Variables|Default|GetPaperSprite1)))

(fn ConstructionScript
  (|CallParentFunction))