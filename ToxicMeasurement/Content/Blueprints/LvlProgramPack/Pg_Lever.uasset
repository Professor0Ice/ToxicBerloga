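; Lever object from the level programming pack that reports its use to the player's OS widget.
; Interaction rotates the sprite half a turn and passes the lever's name to the Levers function on that widget, reached through the TT_Cum pawn's HUD.
; Podsvetka toggles a green highlight on the sprite.
; LoadInfoObj exposes name and image, while LoadInfoProg exposes its condition, action and interaction data.
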(event EventInteraction
  (Transformation|AddRelativeRotation (Variables|Default|GetPaperSprite) "0.000000,180.000000,0.000000" false false)
  (Default|Levers (Variables|/Game/Blueprints/Character/Player/OS_hud.OS_hud_C|GetOS_Widget (Variables|/Game/Blueprints/Character/Player/TT_Cum.TT_Cum_C|GetHUD (.AsTT%20Cum (Utilities|Casting|CastToTT_Cum (Game|Player|GetPlayerPawn 0))))) (Utilities|String|ToString(Text) (Variables|Default|GetName))))

(event EventPodsvetka
  (params (Yes/No :type Boolean))
  (Sprite|SetSpriteColor (Variables|Default|GetPaperSprite) (Math|Color|SelectColor "(R=0.034755,G=1.000000,B=0.000000,A=1.000000)" "(R=1.000000,G=1.000000,B=1.000000,A=1.000000)" Yes/No)))

(fn ConstructionScript)

(fn LoadInfoObj
  (return (Utilities|String|ToString(Text) (Variables|Default|GetName)) (Variables|Default|GetImg)))

(fn LoadInfoProg
  (return (Variables|Default|GetUsl) (Variables|Default|GetDeistv) (Variables|Default|GetVsaimodeistv)))