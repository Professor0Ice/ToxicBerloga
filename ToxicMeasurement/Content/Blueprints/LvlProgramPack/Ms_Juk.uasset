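; Ms_Juk is a patrolling Paper2D beetle hazard that knocks the player away and disrupts them with random HUD commands.
; A timeline moves it by Speed, and it reverses when its probe trace finds nothing or its box overlaps WorldStatic.
; Player contact launches them randomly left or right and, behind a two-second Gate cooldown, queues commands.
; Another timeline spends that queue on random OSWidget ControlBee calls.
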(event OnComponentBeginOverlap(Box)
  (params (OverlappedComponent :type Primitive%20Component%20Object%20Reference) (OtherActor :type Actor%20Object%20Reference) (OtherComp :type Primitive%20Component%20Object%20Reference) (OtherBodyIndex :type Integer) (bFromSweep :type Boolean) (SweepResult :type Hit%20Result%20Structure%20%28by%20ref%29))
  (if (Utilities|Enum|Equal(Enum) (Collision|GetCollisionObjectType OtherComp) "ECC_WorldStatic")
    (CallFunction|RotateT)
    (else
      (bind _astt_player (Utilities|Casting|CastToTT_Player OtherActor))
      (Character|LaunchCharacter _astt_player (Math|Vector|MakeVector (* (* (Math|Random|RandomFloatinRange 1.0 1.25) (Utilities|Select :Index (Math|Random|RandomIntegerinRange 0 1) :Option%200 -1 :Option%201 1)) 3e+02) 0.0 1e+02) false false)
      (Audio|PlaySound2D "/Game/Sound/prujina.prujina" 1.0 1.0 0.0 0 0)
      (Utilities|FlowControl|Gate false :!label _label
        (:Exit
          (Utilities|FlowControl|Sequence
            (:then_0
              (Utilities|FlowControl|Delay 2.0)
              (goto _label Open))
            (:then_1
              (Variables|Default|SetColC (+ (Variables|Default|GetCommandO) (Variables|Default|GetColC))))
            (:then_2
              (goto _label Close))))))))

(event OnComponentHit(PaperFlipbook)
  (params (HitComponent :type Primitive%20Component%20Object%20Reference) (OtherActor :type Actor%20Object%20Reference) (OtherComp :type Primitive%20Component%20Object%20Reference) (NormalImpulse :type Vector :default "0, 0, 0") (Hit :type Hit%20Result%20Structure%20%28by%20ref%29))
  (bind _astt_player (Utilities|Casting|CastToTT_Player OtherActor))
  (Character|LaunchCharacter _astt_player (Math|Vector|MakeVector (* (* (Math|Random|RandomFloatinRange 1.0 1.25) (Utilities|Select :Index (Math|Random|RandomIntegerinRange 0 1) :Option%200 -1 :Option%201 1)) 3e+02) 0.0 1e+02) false false)
  (Audio|PlaySound2D "/Game/Sound/prujina.prujina" 1.0 1.0 0.0 0 0)
  (Utilities|FlowControl|Gate false :!label _label
    (:Exit
      (Utilities|FlowControl|Sequence
        (:then_0
          (Utilities|FlowControl|Delay 2.0)
          (goto _label Open))
        (:then_1
          (Variables|Default|SetColC (+ (Variables|Default|GetCommandO) (Variables|Default|GetColC))))
        (:then_2
          (goto _label Close))))))

(event Custom|RotateT
  (Transformation|AddLocalRotation (Variables|Default|GetPaperFlipbook) "0.000000,180.000000,0.000000" false false)
  (Variables|Default|SetSpeed (* (Variables|Default|GetSpeed) -1.0))
  (Variables|Default|SetProv (* (Variables|Default|GetProv) "-1.000000,0.000000,1.000000")))

(event EventBeginPlay
  (Utilities|FlowControl|Sequence
    (:then_0
      (Utilities|FlowControl|Delay 1.0)
      (Variables|Default|SetOS%20Widget (Variables|/Game/Blueprints/Character/Player/OS_hud.OS_hud_C|GetOS_Widget (Variables|/Game/Blueprints/Character/Player/TT_Cum.TT_Cum_C|GetHUD (.AsTT%20Cum (Utilities|Casting|CastToTT_Cum (Game|Player|GetPlayerPawn 0))))))
      (Timeline|RandCommand Play
        (:Com
          (if (!= (Variables|Default|GetColC) 0)
            (Default|ControlBee (Variables|Default|GetOS%20Widget) (Utilities|Select :Index (Math|Random|RandomIntegerinRange 0 3) :Option%200 "NewEnumerator0" :Option%201 "NewEnumerator1" :Option%202 "NewEnumerator2" :Option%203 "NewEnumerator3"))
            (Variables|Default|SetColC (- (Variables|Default|GetColC) 1))))))
    (:then_1
      (Timeline|beg Play
        (:Update
          (Transformation|AddActorLocalOffset (Math|Vector|MakeVector (Variables|Default|GetSpeed) 0.0 0.0) false false))))))

(event EventTick
  (params (DeltaSeconds :type Float%20%28single-precision%29))
  (bind _paperflipbook (Variables|Default|GetPaperFlipbook))
  (bind _returnvalue (Transformation|GetWorldLocation _paperflipbook))
  (bind _returnvalue_2 (Collision|LineTraceForObjects _returnvalue (+ _returnvalue (Variables|Default|GetProv)) (Variables|Default|GetObject%20Types) false 0 "None"))
  (if (not _returnvalue_2)
    (CallFunction|RotateT)))

(fn ConstructionScript)