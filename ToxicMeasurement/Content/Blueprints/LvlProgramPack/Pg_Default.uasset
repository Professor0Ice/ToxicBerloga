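; Pg_Default is a sprite-based level program object, apparently the default one in LvlProgramPack, that serves its configuration to other code.
; Getter functions return stored variables: name and image, parameter type and timer range, conditions, actions and interactions, OS object, and signal type.
; The Podsvetka event toggles a highlight by tinting the Paper sprite with the highlight color or resetting it to white.
; It has no other logic, and its construction script is empty.
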(event EventPodsvetka
  (params (Yes/No :type Boolean))
  (Sprite|SetSpriteColor (Variables|Default|GetPaperSprite) (Math|Color|SelectColor (Variables|Default|GetColorPodsvetka) "(R=1.000000,G=1.000000,B=1.000000,A=1.000000)" Yes/No)))

(fn ConstructionScript)

(fn LoadInfoObj
  (return (Utilities|String|ToString(Text) (Variables|Default|GetName)) (Variables|Default|GetImg)))

(fn LoadInfoParam
  (return (Variables|Default|GetParametrType) (Variables|Default|GetTimer_Min/Max)))

(fn LoadInfoProg
  (return (Variables|Default|GetUsl) (Variables|Default|GetDeistv) (Variables|Default|GetVsaimodeistv)))

(fn LoadOsObj
  (return (Variables|Default|GetOSobject?)))

(fn TypeSignal
  (return (Variables|Default|GetTypeSignal_0)))