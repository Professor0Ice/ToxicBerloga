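; Programmable spike hazard (Shiep) that restarts the current level when the player hits its sprite while it is active.
; ShiepSignal either toggles the active state or sets it directly.
; Podsvetka highlights the sprite by tinting it green or resetting it to white.
; LoadInfoObj and LoadInfoProg expose its name, image, conditions and actions.
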(event OnComponentHit(PaperSprite)
  (params (HitComponent :type Primitive%20Component%20Object%20Reference) (OtherActor :type Actor%20Object%20Reference) (OtherComp :type Primitive%20Component%20Object%20Reference) (NormalImpulse :type Vector :default "0, 0, 0") (Hit :type Hit%20Result%20Structure%20%28by%20ref%29))
  (if (Variables|Default|GetState)
    (Utilities|Casting|CastToTT_Player OtherActor)
    (bind _returnvalue (Game|GetCurrentLevelName true))
    (Game|OpenLevel(byName) (Utilities|String|StringToName _returnvalue))))

(event EventPodsvetka
  (params (Yes/No :type Boolean))
  (Sprite|SetSpriteColor (Variables|Default|GetPaperSprite) (Math|Color|SelectColor "(R=0.034755,G=1.000000,B=0.000000,A=1.000000)" "(R=1.000000,G=1.000000,B=1.000000,A=1.000000)" Yes/No)))

(event EventShiepSignal
  (params (SmenMode :type Boolean) (On/Off :type Boolean))
  (if SmenMode
    (if (Variables|Default|GetState)
      (Variables|Default|SetState false)
      (else
        (Variables|Default|SetState true)))
    (else
      (Variables|Default|SetState On/Off))))

(fn ConstructionScript)

(fn LoadInfoObj
  (return (Utilities|String|ToString(Text) (Variables|Default|GetName)) (Variables|Default|GetImg)))

(fn LoadInfoProg
  (return (Variables|Default|GetUsl) (Variables|Default|GetDeistv) 0))