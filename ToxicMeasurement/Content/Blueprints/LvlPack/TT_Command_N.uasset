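; TT_Command_N is a level trigger actor that represents one command from the Vib enum: up, down, right, left, hit or finish.
; On BeginPlay it creates a NaprTxt widget in its widget component and labels it with the Russian word for that command.
; When a TT_Player overlaps its Box, it passes Vib to Deistvo on the HUD's OSWidget, reached through the TT_Cum player pawn.
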(event OnComponentBeginOverlap(Box)
  (params (OverlappedComponent :type Primitive%20Component%20Object%20Reference) (OtherActor :type Actor%20Object%20Reference) (OtherComp :type Primitive%20Component%20Object%20Reference) (OtherBodyIndex :type Integer) (bFromSweep :type Boolean) (SweepResult :type Hit%20Result%20Structure%20%28by%20ref%29))
  (Utilities|Casting|CastToTT_Player OtherActor)
  (Utilities|FlowControl|Sequence
    (:then_0
      (Default|Deistvo (Variables|/Game/Blueprints/Character/Player/OS_hud.OS_hud_C|GetOS_Widget (Variables|/Game/Blueprints/Character/Player/TT_Cum.TT_Cum_C|GetHUD (.AsTT%20Cum (Utilities|Casting|CastToTT_Cum (Game|Player|GetPlayerPawn 0))))) (Variables|Default|GetVib)))))

(event EventBeginPlay
  (bind _returnvalue (UserInterface|CreateWidget "/Game/Blueprints/LvlPack/NaprTxt.NaprTxt_C"))
  (bind _output_get (Variables|Default|SetWidgTXT _returnvalue))
  (UserInterface|SetWidget (Variables|Default|GetWidget) _output_get)
  (switch Utilities|FlowControl|Switch|SwitchonDeistvBee (Variables|Default|GetVib)
    (:NewEnumerator0
      (Variables|/Game/Blueprints/LvlPack/NaprTxt.NaprTxt_C|SettextTr (Variables|Default|GetWidgTXT) "Вверх"))
    (:NewEnumerator1
      (Variables|/Game/Blueprints/LvlPack/NaprTxt.NaprTxt_C|SettextTr (Variables|Default|GetWidgTXT) "Вниз"))
    (:NewEnumerator2
      (Variables|/Game/Blueprints/LvlPack/NaprTxt.NaprTxt_C|SettextTr (Variables|Default|GetWidgTXT) "Вправо"))
    (:NewEnumerator3
      (Variables|/Game/Blueprints/LvlPack/NaprTxt.NaprTxt_C|SettextTr (Variables|Default|GetWidgTXT) "Влево"))
    (:NewEnumerator4
      (Variables|/Game/Blueprints/LvlPack/NaprTxt.NaprTxt_C|SettextTr (Variables|Default|GetWidgTXT) "Удар"))
    (:NewEnumerator5
      (Variables|/Game/Blueprints/LvlPack/NaprTxt.NaprTxt_C|SettextTr (Variables|Default|GetWidgTXT) "Финиш"))))

(fn ConstructionScript)